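; Sliding door Blueprint that the player opens with E while input is enabled by its trigger volume.
; Opening requires the overlapping actor to be a ThirdPersonCharacter with DoorIsOpen set, then activates two steam effects.
; A timeline lerps the door mesh's relative location from closed to open.
; Leaving the trigger disables input and reverses the timeline to close the door.
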(event `Key|E`
  (params (Key :type "Key Structure"))
  (:`Pressed`
    (bind _asthird_person_character (cast `/Game/ThirdPersonBP/Blueprints/ThirdPersonCharacter` (stale `self.Trigger.OnComponentBeginOverlap` OtherActor)))
    (if (`/Game/ThirdPersonBP/Blueprints/ThirdPersonCharacter.DoorIsOpen` _asthird_person_character)
      (`ActorComponent.Activate` (`self.SteamDoor`) false)
      (`ActorComponent.Activate` (`self.SteamDoor2`) false)
      (bind (_direction _doorposition) (`Timeline|Timeline_0` :!label _label)
        (:`Update`
          (`SceneComponent.K2_SetRelativeLocation` (`self.Door_Small_A`) (`KismetMathLibrary.VLerp` (`self.DoorClosed`) (`self.DoorOpen`) _doorposition) false false))))))

(event `self.Trigger.OnComponentBeginOverlap`
  (params (OverlappedComponent :type "PrimitiveComponent Object Reference") (OtherActor :type "Actor Object Reference") (OtherComp :type "PrimitiveComponent Object Reference") (OtherBodyIndex :type Integer) (bFromSweep :type Boolean) (SweepResult :type "HitResult Structure (by ref)"))
  (`self.EnableInput` (`GameplayStatics.GetPlayerController` 0)))

(event `self.Trigger.OnComponentEndOverlap`
  (params (OverlappedComponent :type "PrimitiveComponent Object Reference") (OtherActor :type "Actor Object Reference") (OtherComp :type "PrimitiveComponent Object Reference") (OtherBodyIndex :type Integer))
  (`self.DisableInput` (`GameplayStatics.GetPlayerController` 0))
  (goto _label :!via `Reverse`))

(fn `UserConstructionScript`)